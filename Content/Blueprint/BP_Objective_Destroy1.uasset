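; BP_Objective_Destroy1 is a destructible tutorial objective that oscillates between two points offset either side of its start location.
; Movement uses VInterpTo in delay-driven loops, with two Gates switching targets within a tolerance radius.
; Hit plays effects, destroys the actor and decrements a BP_GameMode counter, completing the Room11 mission at zero.
; When NoVisible is set, Tick keeps it hidden and non-collidable until the Room10 mission completes.
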(event EventBeginPlay
  (bind _returnvalue (Transformation|GetActorLocation))
  (bind _returnvalue_2 (Transformation|GetActorLocation))
  (bind _returnvalue_3 (Transformation|GetActorLocation))
  (bind _ychange (Variables|Default|GetYChange))
  (bind _zchange (Variables|Default|GetZChange))
  (bind _xchange (Variables|Default|GetXChange))
  ;[1 1 1] Movimiento oscilatorio relativo a posición inicial usando interpolación
  ;;[1 1 1] Setear puntos de inicio y fin
  (Variables|Default|SetTarget1 (Math|Vector|MakeVector (- (.x _returnvalue) _xchange) (- (.y _returnvalue) _ychange) (- (.z _returnvalue) _zchange)))
  (Variables|Default|SetTarget2 (Math|Vector|MakeVector (+ (.x _returnvalue) _xchange) (+ (.y _returnvalue) _ychange) (+ (.z _returnvalue) _zchange)))
  ;;[1 1 1] Ir a Target1
  (Utilities|FlowControl|Sequence ; Ir a Target1
    (:then_0
      (Transformation|SetActorLocation (Math|Interpolation|VInterpTo _returnvalue_2 (Variables|Default|GetTarget1) (Utilities|Time|GetWorldDeltaSeconds) (Variables|Default|GetInterpSpeed)) false false :!label _label)
      (Utilities|FlowControl|Delay (Variables|Default|GetRefresh%28secs%29))
      (Utilities|FlowControl|Sequence ; Luego de mover, verificar si llegó a Target1
        (:then_0
          (Utilities|FlowControl|Gate true :!label _label_2 ; Cambio entre ir a Target1 y Target2
            (:Exit
              (goto _label))))
        (:then_1
          (if (Math|Vector|Equal(Vector) _returnvalue_2 (Variables|Default|GetTarget1) (Variables|Default|GetTargetCollisionRadius))
            (Utilities|FlowControl|Sequence ; Dejar de ir a Target1
              (:then_0
                (goto _label_2 Close))
              (:then_1
                ;;[1 1 1] Ir a Target2
                (Utilities|FlowControl|Sequence ; Ir a Target2
                  (:then_0
                    (Transformation|SetActorLocation (Math|Interpolation|VInterpTo _returnvalue_3 (Variables|Default|GetTarget2) (Utilities|Time|GetWorldDeltaSeconds) (Variables|Default|GetInterpSpeed)) false false :!label _label_3)
                    (Utilities|FlowControl|Delay (Variables|Default|GetRefresh%28secs%29))
                    (Utilities|FlowControl|Sequence ; Luego de mover, verificar si llegó a Target2
                      (:then_0
                        (Utilities|FlowControl|Gate true :!label _label_4
                          (:Exit
                            (goto _label_3))))
                      (:then_1
                        (if (Math|Vector|Equal(Vector) _returnvalue_3 (Variables|Default|GetTarget2) (Variables|Default|GetTargetCollisionRadius)) ; Si llegó a Target2, Loop
                          (Utilities|FlowControl|Sequence ; Dejar de ir a Target2. Ir a Target1
                            (:then_0
                              (goto _label_4 Close))
                            (:then_1
                              (goto _label))
                            (:then_2
                              (goto _label_2 Open)))))))
                  (:then_1
                    (goto _label_4 Open)))))))))
    (:then_1
      (goto _label_2 Open))))

(event EventTick
  (params (DeltaSeconds :type Float%20%28single-precision%29))
  (bind _novisible (Variables|Default|GetNoVisible))
  (bind _box (Variables|Default|GetBox))
  ;[1 1 1] Actor visible cuando se completa la primera misión
  (if _novisible
    (bind _asbp_game_mode (Utilities|Casting|CastToBP_GameMode (Game|GetGameMode)))
    (Rendering|SetActorHiddenInGame (not (Variables|/Game/Blueprint/GameMode/BP_GameMode.BP_GameMode_C|GetmissionCom_tuto1_room1_0 _asbp_game_mode)))
    (if (not (Variables|/Game/Blueprint/GameMode/BP_GameMode.BP_GameMode_C|GetmissionCom_tuto1_room1_0 _asbp_game_mode))
      (Collision|SetCollisionEnabled _box "NoCollision")
      (else
        (Collision|SetCollisionEnabled _box "QueryOnly")))
    (else
      (Rendering|SetActorHiddenInGame _novisible)
      (Collision|SetCollisionEnabled (Variables|Default|GetBox) "QueryOnly"))))

(event Collision|EventHit
  (params (MyComp :type Primitive%20Component%20Object%20Reference) (Other :type Actor%20Object%20Reference) (OtherComp :type Primitive%20Component%20Object%20Reference) (bSelfMoved :type Boolean) (HitLocation :type Vector :default "0, 0, 0") (HitNormal :type Vector :default "0, 0, 0") (NormalImpulse :type Vector :default "0, 0, 0") (Hit :type Hit%20Result%20Structure%20%28by%20ref%29))
  (bind _returnvalue (Transformation|GetActorLocation))
  ;[1 1 1] Disparo Evento
  (bind _asbp_game_mode (Utilities|Casting|CastToBP_GameMode (Game|GetGameMode)))
  (Audio|PlaySoundatLocation (Variables|Default|GetsonidoDestroy) _returnvalue)
  (Effects|SpawnEmitteratLocation (Variables|Default|GetParticleDestroy) _returnvalue "0, 0, 0" (Variables|Default|GetparticleScale))
  (Variables|/Game/Blueprint/GameMode/BP_GameMode.BP_GameMode_C|SetTuto1ShootObj _asbp_game_mode (- (Variables|/Game/Blueprint/GameMode/BP_GameMode.BP_GameMode_C|GetTuto1ShootObj _asbp_game_mode) 1))
  (Actor|DestroyActor)
  ;[1 1 1] Sonido al completar objetivos destruibles
  (if (<= (Variables|/Game/Blueprint/GameMode/BP_GameMode.BP_GameMode_C|GetTuto1ShootObj _asbp_game_mode) 0)
    (if (Variables|Default|Getuna_vez_overlap)
      (Variables|Default|Setuna_vez_overlap false)
      (Audio|PlaySoundatLocation "/Game/Audio/Au_miniQuestComplete.Au_miniQuestComplete" (Transformation|GetActorLocation))
      (bind _asbp_game_mode_2 (Utilities|Casting|CastToBP_GameMode (Game|GetGameMode)))
      (Variables|/Game/Blueprint/GameMode/BP_GameMode.BP_GameMode_C|SetmissionCom_tuto1_room1_1 _asbp_game_mode_2 true)
      (if (Variables|/Game/Blueprint/GameMode/BP_GameMode.BP_GameMode_C|GetmissionCom_tuto1_room1_0 _asbp_game_mode_2)
        (Audio|PlaySound2D "/Game/Audio/Au_QuestComplete.Au_QuestComplete")))))

(fn ConstructionScript)