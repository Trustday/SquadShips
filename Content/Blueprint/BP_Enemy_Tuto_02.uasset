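; BP_Enemy_Tuto_02 is a tutorial enemy Blueprint that combines flight-style movement with a looping two-point AI patrol.
; Tick sweeps the actor forward by ForwardSpeed and rotates it by roll, pitch and yaw speeds.
; The Patrol event runs AI MoveTo to Target1, then Target2, with short delays and debug prints, and calls itself again on success.
; BeginPlay is empty, and nothing in this file starts Patrol.
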(event Custom|Patrol
  (Development|PrintString "Patrullando")
  (AI|AIMoveTo self "0, 0, 0" (Variables|Default|GetTarget1) 5.0 false
    (:OnSuccess
      (Utilities|FlowControl|Delay 0.2)
      (AI|AIMoveTo self "0, 0, 0" (Variables|Default|GetTarget2) 5.0 false
        (:OnSuccess
          (Utilities|FlowControl|Delay 0.2)
          (Development|PrintString "Termino de patrullar")
          (CallFunction|Patrol))))))

(event Collision|EventActorBeginOverlap
  (params (OtherActor :type Actor%20Object%20Reference)))

(event EventTick
  (params (DeltaSeconds :type Float%20%28single-precision%29))
  (bind _returnvalue (Utilities|Time|GetWorldDeltaSeconds))
  (Transformation|AddActorLocalOffset (Math|Vector|MakeVector (* DeltaSeconds (Variables|Default|GetForwardSpeed)) 0.0 0.0) true false) ; Sweep plane forwards
  (Transformation|AddActorLocalRotation (Math|Rotator|MakeRotator (* _returnvalue (Variables|Default|GetRollSpeed)) (* _returnvalue (Variables|Default|GetPitchSpeed)) (* _returnvalue (Variables|Default|GetYawSpeed))) false false))

(event EventBeginPlay)

(fn ConstructionScript)