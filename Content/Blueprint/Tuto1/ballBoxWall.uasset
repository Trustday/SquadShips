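; Tutorial ball-target wall that spins slowly in yaw every tick and shatters after being hit by a noGravityBall.
; The first ball hit turns on physics for the Wall and swaps it to a transparent purple material.
; A later hit from anything except noGravityObj plays glass hit and break sounds with delays, then destroys the actor.
; Before any ball hit, other objects only trigger a wrong-hit sound, and noGravityObj hits are ignored.
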(event EventBeginPlay)

(event Collision|EventActorBeginOverlap
  (params (OtherActor :type Actor%20Object%20Reference)))

(event EventTick
  (params (DeltaSeconds :type Float%20%28single-precision%29))
  (bind _defaultsceneroot (Variables|Default|GetDefaultSceneRoot))
  (bind _returnvalue (Transformation|GetWorldRotation _defaultsceneroot))
  ;[1 1 1] Rotación
  (Transformation|SetWorldRotation _defaultsceneroot (Math|Rotator|MakeRotator (.roll _returnvalue) (.pitch _returnvalue) (+ (.yaw _returnvalue) -0.5)) false false))

(event Collision|EventHit
  (params (MyComp :type Primitive%20Component%20Object%20Reference) (Other :type Actor%20Object%20Reference) (OtherComp :type Primitive%20Component%20Object%20Reference) (bSelfMoved :type Boolean) (HitLocation :type Vector :default "0, 0, 0") (HitNormal :type Vector :default "0, 0, 0") (NormalImpulse :type Vector :default "0, 0, 0") (Hit :type Hit%20Result%20Structure%20%28by%20ref%29))
  ;[1 1 1] Event Hit: Comportamiento y sonidos
  (Utilities|Casting|CastTonoGravityBall Other
    (:then
      (if (Variables|Default|GetballHit) ; Si golpea pelota
        (if (Variables|Default|GetplaySoundGlassHit) :!label _label ; Si había golpeado antes pelota
          (Variables|Default|SetplaySoundGlassHit false)
          (else
            (Utilities|FlowControl|Delay 0.5)))
        (Audio|PlaySound2D "/Game/Audio/Au_glassHit.Au_glassHit")
        (Utilities|FlowControl|Delay 1.5)
        (Audio|PlaySound2D "/Game/Audio/Au_BreakGlass.Au_BreakGlass")
        (Actor|DestroyActor)
        (else
          (Variables|Default|SetballHit true) ; Si no había golpeado antes pelota
          (Physics|SetSimulatePhysics (Variables|Default|Getwall) true)
          (Rendering|Material|SetMaterial (Variables|Default|Getwall) 0 "/Game/Meshes/Materials/MAT_PurpleTrans.MAT_PurpleTrans"))))
    (:CastFailed
      (Utilities|Casting|CastTonoGravityObj Other ; Si no es pelota
        (:CastFailed
          (if (Variables|Default|GetballHit) ; Si no es este mismo obj
            (goto _label)
            (else
              (if (Variables|Default|GetplaySoundWrong) ; Si no había golpeado antes pelota
                (Variables|Default|SetplaySoundWrong false)
                (else
                  (Utilities|FlowControl|Delay 0.2)))
              (Audio|PlaySound2D "/Game/Audio/Au_wrongMode.Au_wrongMode"))))))))

(fn ConstructionScript)