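; Destructible secret crystal that the player character (BP_Main) hits to register a found secret.
; On begin play it destroys itself if the GlobalGameInstance secret count already covers it, using actor tag "1" to choose between the first and second secret threshold.
; A hit from BP_Main on the destructible component plays a sound and increments that count, with the UnaVez flag limiting this to once.
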(event OnComponentHit(DestructibleComponent)
  (params (HitComponent :type Primitive%20Component%20Object%20Reference) (OtherActor :type Actor%20Object%20Reference) (OtherComp :type Primitive%20Component%20Object%20Reference) (NormalImpulse :type Vector :default "0, 0, 0") (Hit :type Hit%20Result%20Structure%20%28by%20ref%29))
  ;[1 1 1] Sumar uno a secretos y play sound
  (if (Variables|Default|GetunaVez)
    (Utilities|Casting|CastToBP_Main OtherActor)
    (Audio|PlaySound2D "/Game/Audio/Au_SecretFound.Au_SecretFound")
    (bind _asglobal_game_instance (Utilities|Casting|CastToGlobalGameInstance (Game|GetGameInstance)))
    (Math|Integer|IncrementInt (Variables|/Game/Blueprint/GameMode/GlobalGameInstance.GlobalGameInstance_C|GetsecretsFound _asglobal_game_instance)
      (:%20%20
        (Variables|Default|SetunaVez false)))))

(event EventBeginPlay
  ;[1 1 1] Destruir si ya se obtuvo el secreto
  (if (Actor|ActorHasTag "1")
    (bind _asglobal_game_instance (Utilities|Casting|CastToGlobalGameInstance (Game|GetGameInstance)))
    (if (>= (Variables|/Game/Blueprint/GameMode/GlobalGameInstance.GlobalGameInstance_C|GetsecretsFound _asglobal_game_instance) 1)
      (Actor|DestroyActor))
    (else
      (bind _asglobal_game_instance_2 (Utilities|Casting|CastToGlobalGameInstance (Game|GetGameInstance)))
      (if (>= (Variables|/Game/Blueprint/GameMode/GlobalGameInstance.GlobalGameInstance_C|GetsecretsFound _asglobal_game_instance_2) 2)
        (Actor|DestroyActor)))))

(event Collision|EventActorBeginOverlap
  (params (OtherActor :type Actor%20Object%20Reference)))

(event EventTick
  (params (DeltaSeconds :type Float%20%28single-precision%29)))

(fn ConstructionScript)