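; Tutorial sign actor that is revealed when both Room 1 missions are complete and triggers the room's closing dialogue.
; Tick polls BP_GameMode for the mission flags, then once unhides the actor and starts the dialogue, also toggling its text components if tagged "Not".
; The dialogue widget shows two timed text and portrait lines, and Tick removes it whenever Room 2 has been entered.
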(event Custom|DialogoFinRoom1
  ;[1 1 1] Dialogo Final Mision 1 Room1
  (bind _returnvalue (Game|ConstructObjectfromClass "/Game/UI/Dialogos/BP_Dialogo_Plantilla_Lvl.BP_Dialogo_Plantilla_Lvl_C" (Game|GetPlayerController 0)))
  (bind _output_get (Variables|Default|SetDialogoFinalRoom1 _returnvalue))
  (UserInterface|Viewport|AddtoViewport _output_get 0)
  (Variables|/Game/UI/Dialogos/BP_Dialogo_Plantilla_Lvl.BP_Dialogo_Plantilla_Lvl_C|SetDialogue_Text _returnvalue (Variables|Default|GetDialogoFinal_Room1_1))
  (Variables|/Game/UI/Dialogos/BP_Dialogo_Plantilla_Lvl.BP_Dialogo_Plantilla_Lvl_C|SetTextura _returnvalue (Variables|Default|GetImagenKai))
  (Utilities|FlowControl|Delay 5.0)
  (Variables|/Game/UI/Dialogos/BP_Dialogo_Plantilla_Lvl.BP_Dialogo_Plantilla_Lvl_C|SetDialogue_Text _returnvalue (Variables|Default|GetDialogoFinal_Room1_2))
  (Variables|/Game/UI/Dialogos/BP_Dialogo_Plantilla_Lvl.BP_Dialogo_Plantilla_Lvl_C|SetTextura _returnvalue (Variables|Default|GetImagenIA))
  (Utilities|FlowControl|Delay 3.0)
  (Widget|RemovefromParent (Variables|Default|GetDialogoFinalRoom1)))

(event EventTick
  (params (DeltaSeconds :type Float%20%28single-precision%29))
  ;[1 1 1] Actor visible cuando se completa ROOM1
  (bind _asbp_game_mode (Utilities|Casting|CastToBP_GameMode (Game|GetGameMode)))
  (if (Variables|/Game/Blueprint/GameMode/BP_GameMode.BP_GameMode_C|GetenteredRoom2 _asbp_game_mode)
    (Widget|RemovefromParent (Variables|Default|GetDialogoFinalRoom1)))
  (if (Variables|Default|GetunaVez)
    (bind _asbp_game_mode_2 (Utilities|Casting|CastToBP_GameMode (Game|GetGameMode)))
    (if (and (Variables|/Game/Blueprint/GameMode/BP_GameMode.BP_GameMode_C|GetmissionCom_tuto1_room1_0 _asbp_game_mode_2) (Variables|/Game/Blueprint/GameMode/BP_GameMode.BP_GameMode_C|GetmissionCom_tuto1_room1_1 _asbp_game_mode_2))
      (Rendering|SetActorHiddenInGame (not (and (Variables|/Game/Blueprint/GameMode/BP_GameMode.BP_GameMode_C|GetmissionCom_tuto1_room1_0 _asbp_game_mode_2) (Variables|/Game/Blueprint/GameMode/BP_GameMode.BP_GameMode_C|GetmissionCom_tuto1_room1_1 _asbp_game_mode_2))))
      (CallFunction|DialogoFinRoom1)
      (Variables|Default|SetunaVez false)
      ;[1 1 1] Cambiar visibilidad del mensaje con Tag [Not]
      (if (Actor|ActorHasTag "Not")
        (Rendering|ToggleVisibility (Variables|Default|GetText[NEXT]) false)
        (Rendering|ToggleVisibility (Variables|Default|GetText[ROOM]) false)
        (Rendering|ToggleVisibility (Variables|Default|GetText[GO%20THE]) false)
        (Rendering|ToggleVisibility (Variables|Default|GetText[OTHER%20WAY]) false)))))

(fn ConstructionScript)