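; BP_NRT_1-3 is a tutorial trigger actor that marks the player's first entry into room 3.
; On overlap with BP_Main, it sets the GameMode's EnteredRoom3 flag and briefly raises ShowMisUpd, apparently a mission-update notice.
; It also shows a timed two-part dialogue widget, instructions with the IA portrait, then a response with Kai's, before removing it.
; The GameMode flag and a local UnaVez flag guard against repeats.
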(event Custom|NuevasInstrucciones
  ;[1 1 1] Dialogo EntrarRoom 3
  (if (not (Variables|Default|GetunaVez))
    (bind _returnvalue (Game|ConstructObjectfromClass "/Game/UI/Dialogos/BP_Dialogo_Plantilla_Lvl.BP_Dialogo_Plantilla_Lvl_C" (Game|GetPlayerController 0)))
    (bind _output_get (Variables|Default|SetDialogoInstrucciones _returnvalue))
    (UserInterface|Viewport|AddtoViewport _output_get 0)
    (Variables|/Game/UI/Dialogos/BP_Dialogo_Plantilla_Lvl.BP_Dialogo_Plantilla_Lvl_C|SetDialogue_Text _returnvalue (Variables|Default|GetInstrucciones))
    (Variables|/Game/UI/Dialogos/BP_Dialogo_Plantilla_Lvl.BP_Dialogo_Plantilla_Lvl_C|SetTextura _returnvalue (Variables|Default|GetImagen%20IA))
    (Utilities|FlowControl|Delay 5.0)
    (Variables|/Game/UI/Dialogos/BP_Dialogo_Plantilla_Lvl.BP_Dialogo_Plantilla_Lvl_C|SetDialogue_Text _returnvalue (Variables|Default|GetRespuesta))
    (Variables|/Game/UI/Dialogos/BP_Dialogo_Plantilla_Lvl.BP_Dialogo_Plantilla_Lvl_C|SetTextura _returnvalue (Variables|Default|GetImagen%20Kai))
    (Utilities|FlowControl|Delay 2.0)
    (Widget|RemovefromParent (Variables|Default|GetDialogoInstrucciones))
    (Variables|Default|SetunaVez true)))

(event EventBeginPlay)

(event EventTick
  (params (DeltaSeconds :type Float%20%28single-precision%29)))

(event Collision|EventActorBeginOverlap
  (params (OtherActor :type Actor%20Object%20Reference))
  ;[1 1 1] Set entered room 3
  (Utilities|Casting|CastToBP_Main OtherActor)
  (bind _asbp_game_mode (Utilities|Casting|CastToBP_GameMode (Game|GetGameMode)))
  (if (not (Variables|/Game/Blueprint/GameMode/BP_GameMode.BP_GameMode_C|GetenteredRoom3 _asbp_game_mode))
    (Variables|/Game/Blueprint/GameMode/BP_GameMode.BP_GameMode_C|SetenteredRoom3 _asbp_game_mode true)
    (Variables|/Game/Blueprint/GameMode/BP_GameMode.BP_GameMode_C|SetshowMisUpd _asbp_game_mode true)
    (CallFunction|NuevasInstrucciones)
    (Utilities|FlowControl|Delay 2.5)
    (Variables|/Game/Blueprint/GameMode/BP_GameMode.BP_GameMode_C|SetshowMisUpd _asbp_game_mode false)))

(fn ConstructionScript
  (|CallParentFunction))