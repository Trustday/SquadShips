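; BP_NextRoom2Text is a tutorial sign actor that is revealed in game once the player completes a room's missions.
; Tick polls two Room 2 mission flags on BP_GameMode, unhides the actor when both are true, then clears UnaVez so it fires only once.
; Instances tagged "Not" also toggle their four text components, flipping between next-room and go-the-other-way wording.
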(event EventBeginPlay)

(event Collision|EventActorBeginOverlap
  (params (OtherActor :type Actor%20Object%20Reference)))

(event EventTick
  (params (DeltaSeconds :type Float%20%28single-precision%29))
  ;[1 1 1] Actor visible cuando se completa ROOM1
  (if (Variables|Default|GetunaVez)
    (bind _asbp_game_mode (Utilities|Casting|CastToBP_GameMode (Game|GetGameMode)))
    (if (and (Variables|/Game/Blueprint/GameMode/BP_GameMode.BP_GameMode_C|GetmissionCom_tuto1_room2_0 _asbp_game_mode) (Variables|/Game/Blueprint/GameMode/BP_GameMode.BP_GameMode_C|GetmissionCom_tuto1_room2_1 _asbp_game_mode))
      (Rendering|SetActorHiddenInGame (not (and (Variables|/Game/Blueprint/GameMode/BP_GameMode.BP_GameMode_C|GetmissionCom_tuto1_room2_0 _asbp_game_mode) (Variables|/Game/Blueprint/GameMode/BP_GameMode.BP_GameMode_C|GetmissionCom_tuto1_room2_1 _asbp_game_mode))))
      (Variables|Default|SetunaVez false)
      ;[1 1 1] Cambiar visibilidad del mensaje con Tag [Not]
      (if (Actor|ActorHasTag "Not")
        (Rendering|ToggleVisibility (Variables|Default|GetText[NEXT]) false)
        (Rendering|ToggleVisibility (Variables|Default|GetText[ROOM]) false)
        (Rendering|ToggleVisibility (Variables|Default|GetText[GO%20THE]) false)
        (Rendering|ToggleVisibility (Variables|Default|GetText[OTHER%20WAY]) false)))))

(fn ConstructionScript)