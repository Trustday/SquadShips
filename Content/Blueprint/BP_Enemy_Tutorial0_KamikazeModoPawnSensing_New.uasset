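; Tutorial flying kamikaze enemy that patrols a loop of four targets, then chases and shoots at BP_Main when PawnSensing spots it.
; Tick drives forward movement; target overlaps re-aim the patrol, while sighting sets a timed chase state that faces the player and fires through a Delay-throttled spawn.
; It explodes on ramming the player, dealing damage, or when Life runs out; destruction updates tutorial and global kill counters.
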(event OnSeePawn(PawnSensing)
  (params (Pawn :type Pawn%20Object%20Reference))
  ;[1 1 1] Logica de seguir
  (Utilities|Casting|CastToBP_Main Pawn)
  (Utilities|FlowControl|Sequence
    (:then_0
      (Variables|Default|SetestadoNave 0))
    (:then_1
      (Utilities|FlowControl|Delay 5.0)
      (Variables|Default|SetestadoNave 1)
      (Transformation|SetActorRotation (Math|Rotator|FindLookatRotation (Transformation|GetWorldLocation (Variables|Default|GetSphere)) (Transformation|GetActorLocation (Variables|Default|Gettarget1)))))))

(event Custom|RestarEnemigos
  ;[1 1 1] Restar Enemigos
  (bind _asbp_game_mode (Utilities|Casting|CastToBP_GameMode (Game|GetGameMode)))
  (bind _result (Math|Integer|DecrementInt (Variables|/Game/Blueprint/GameMode/BP_GameMode.BP_GameMode_C|GetTuto1FlyingEnemies _asbp_game_mode))
    (:%20%20
      ;[1 1 1] Sumar uno a Enemies killed
      (bind _asglobal_game_instance (Utilities|Casting|CastToGlobalGameInstance (Game|GetGameInstance)))
      (Math|Integer|IncrementInt (Variables|/Game/Blueprint/GameMode/GlobalGameInstance.GlobalGameInstance_C|GetenemiesKilled _asglobal_game_instance)
        (:%20%20
          ;[1 1 1] Mini mision complete
          (if (<= _result 0)
            (Audio|PlaySoundatLocation "/Game/Audio/Au_miniQuestComplete.Au_miniQuestComplete" (Transformation|GetActorLocation))))))))

(event Custom|Seguir
  ;[1 1 1] Seguir al player
  (bind _asbp_main (Utilities|Casting|CastToBP_Main (Game|GetPlayerCharacter 0)))
  (Transformation|SetActorRotation (Math|Rotator|FindLookatRotation (Transformation|GetWorldLocation (Variables|Default|GetSphere)) (Transformation|GetActorLocation _asbp_main))))

(event EventDestroyed
  ;[1 1 1] Al destruir
  (CallFunction|RestarEnemigos))

(event EventBeginPlay
  ;[1 1 1] Que al iniciar valla al target 1
  (Transformation|SetActorRotation (Math|Rotator|FindLookatRotation (Transformation|GetWorldLocation (Variables|Default|GetSphere)) (Transformation|GetActorLocation (Variables|Default|Gettarget1)))))

(event EventTick
  (params (DeltaSeconds :type Float%20%28single-precision%29))
  (bind _returnvalue (Utilities|Time|GetWorldDeltaSeconds))
  ;[1 1 1] ON TICK: Apply forward speed and steering rotation
  (Transformation|AddActorLocalOffset (Math|Vector|MakeVector (* DeltaSeconds (Variables|Default|GetCurrent%20forward%20speed)) 0.0 0.0) true false) ; Sweep plane forwards
  (Transformation|AddActorLocalRotation (Math|Rotator|MakeRotator (* _returnvalue (Variables|Default|GetCurrent%20roll%20speed)) (* _returnvalue (Variables|Default|GetCurrent%20pitch%20speed)) (* _returnvalue (Variables|Default|GetCurrent%20yaw%20speed))) false false)
  (switch int (Variables|Default|GetestadoNave)
    (:0
      (CallFunction|Seguir)
      (Utilities|FlowControl|Delay 1.0)
      (Game|SpawnActorfromClass "/Game/Blueprint/BP_2_Primario.BP_2_Primario_C" (Transformation|GetWorldTransform (Variables|Default|GetArrow)) "Undefined" 0 0)
      (Audio|PlaySoundatLocation "/Game/Audio/Au_enemyShoot.Au_enemyShoot" (Transformation|GetActorLocation self)) ; Play firing sound
    )))

(event Game|Damage|EventAnyDamage
  (params (Damage :type Float%20%28single-precision%29) (DamageType :type Damage%20Type%20Object%20Reference) (InstigatedBy :type Controller%20Object%20Reference) (DamageCauser :type Actor%20Object%20Reference))
  (bind _returnvalue (Transformation|GetActorLocation))
  ;[1 1 1] Aplicar Daño
  (bind _output_get (Variables|Default|SetLife (- (Variables|Default|GetLife) Damage)))
  (if (<= _output_get 0.0)
    (Effects|SpawnEmitteratLocation "/Game/StarterContent/Particles/P_Explosion.P_Explosion" _returnvalue)
    (Audio|PlaySoundatLocation "/Game/StarterContent/Audio/Explosion01.Explosion01" _returnvalue)
    (Actor|DestroyActor)))

(event Collision|EventActorBeginOverlap
  (params (OtherActor :type Actor%20Object%20Reference))
  ;[1 1 1] Cambio a un target
  (bind _asbp_target (Utilities|Casting|CastToBP_Target OtherActor))
  (if (Math|Vector|Equal(Vector) (Transformation|GetActorLocation (Variables|Default|Gettarget1)) (Transformation|GetActorLocation _asbp_target) 5e+02)
    (Transformation|SetActorRotation (Math|Rotator|FindLookatRotation (Transformation|GetWorldLocation (Variables|Default|GetSphere)) (Transformation|GetActorLocation (Variables|Default|Gettarget2))))
    (elif (Math|Vector|Equal(Vector) (Transformation|GetActorLocation (Variables|Default|Gettarget2)) (Transformation|GetActorLocation _asbp_target) 5e+02)
      (Transformation|SetActorRotation (Math|Rotator|FindLookatRotation (Transformation|GetWorldLocation (Variables|Default|GetSphere)) (Transformation|GetActorLocation (Variables|Default|Gettarget3))))
      (elif (Math|Vector|Equal(Vector) (Transformation|GetActorLocation (Variables|Default|Gettarget3)) (Transformation|GetActorLocation _asbp_target) 5e+02)
        (Transformation|SetActorRotation (Math|Rotator|FindLookatRotation (Transformation|GetWorldLocation (Variables|Default|GetSphere)) (Transformation|GetActorLocation (Variables|Default|Gettarget4))))
        (elif (Math|Vector|Equal(Vector) (Transformation|GetActorLocation (Variables|Default|Gettarget4)) (Transformation|GetActorLocation _asbp_target) 5e+02)
          (Transformation|SetActorRotation (Math|Rotator|FindLookatRotation (Transformation|GetWorldLocation (Variables|Default|GetSphere)) (Transformation|GetActorLocation (Variables|Default|Gettarget1)))))))))

(event Collision|EventHit
  (params (MyComp :type Primitive%20Component%20Object%20Reference) (Other :type Actor%20Object%20Reference) (OtherComp :type Primitive%20Component%20Object%20Reference) (bSelfMoved :type Boolean) (HitLocation :type Vector :default "0, 0, 0") (HitNormal :type Vector :default "0, 0, 0") (NormalImpulse :type Vector :default "0, 0, 0") (Hit :type Hit%20Result%20Structure%20%28by%20ref%29))
  (bind _returnvalue (Transformation|GetActorLocation))
  ;[1 1 1] Detectar Daño
  (bind _asbp_main (Utilities|Casting|CastToBP_Main Other))
  (Game|Damage|ApplyDamage _asbp_main 75.0 0 0)
  (Effects|SpawnEmitteratLocation "/Game/StarterContent/Particles/P_Explosion.P_Explosion" _returnvalue)
  (Audio|PlaySoundatLocation "/Game/StarterContent/Audio/Explosion01.Explosion01" _returnvalue)
  (Actor|DestroyActor))

(fn ConstructionScript)