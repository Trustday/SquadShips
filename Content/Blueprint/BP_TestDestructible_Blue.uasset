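; BP_TestDestructible_Blue is a destructible objective target that breaks when it receives a Hit event.
; On hit it plays a glass-smash sound, decrements the Objetivos counter on BP_GameMode and destroys itself.
; If that counter reaches zero or below, it also plays a quest-complete sound, gated by the one-shot UnaVezOverlap flag.
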(event EventBeginPlay
  ;[1 1 1] Disparo Evento
)

(event Collision|EventHit
  (params (MyComp :type Primitive%20Component%20Object%20Reference) (Other :type Actor%20Object%20Reference) (OtherComp :type Primitive%20Component%20Object%20Reference) (bSelfMoved :type Boolean) (HitLocation :type Vector :default "0, 0, 0") (HitNormal :type Vector :default "0, 0, 0") (NormalImpulse :type Vector :default "0, 0, 0") (Hit :type Hit%20Result%20Structure%20%28by%20ref%29))
  ;[1 1 1] Disparo Evento
  (bind _asbp_game_mode (Utilities|Casting|CastToBP_GameMode (Game|GetGameMode)))
  (Audio|PlaySoundatLocation "/Game/Audio/au_tinkle-smash-glass.au_tinkle-smash-glass" (Transformation|GetActorLocation))
  (Variables|/Game/Blueprint/BP_GameMode.BP_GameMode_C|SetObjetivos _asbp_game_mode (- (Variables|/Game/Blueprint/BP_GameMode.BP_GameMode_C|GetObjetivos _asbp_game_mode) 1))
  (Actor|DestroyActor)
  ;[1 1 1] Sonido al completar objetivos destruibles
  (if (<= (Variables|/Game/Blueprint/BP_GameMode.BP_GameMode_C|GetObjetivos _asbp_game_mode) 0)
    (if (Variables|Default|Getuna_vez_overlap)
      (Variables|Default|Setuna_vez_overlap false)
      (Audio|PlaySoundatLocation "/Game/Audio/Au_miniQuestComplete.Au_miniQuestComplete" (Transformation|GetActorLocation)))))

(fn ConstructionScript)