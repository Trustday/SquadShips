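; BP_PreGameMode is a game mode Blueprint that starts continuous enemy spawning from two warper actors at BeginPlay.
; It takes the first BP_Warper and first BP_Warper2 found in the level as spawners.
; Looping timers call EnemySpawn2 and Warper2 on them by function name, both at an interval derived from the shared EnemyPerSecond rate.
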(event EventBeginPlay
  ;[1 1 1] Spawn Enemigo 1
  (bind _outactors (Actor|GetAllActorsOfClass "/Game/Blueprint/BP_Warper.BP_Warper_C"))
  (bind _output_get (Variables|Default|SetSpawner (Utilities|Array|Get(acopy) _outactors)))
  (Utilities|Time|SetTimerbyFunctionName _output_get "EnemySpawn2" (/ 1.0 (Variables|Default|GetEnemyPerSecond)) true)
  ;[1 1 1] Spawn Enemigo 2
  (bind _outactors_2 (Actor|GetAllActorsOfClass "/Game/Blueprint/BP_Warper2.BP_Warper2_C"))
  (bind _output_get_2 (Variables|Default|SetSpawner2 (Utilities|Array|Get(acopy) _outactors_2)))
  (Utilities|Time|SetTimerbyFunctionName _output_get_2 "Warper2" (/ 1.0 (Variables|Default|GetEnemyPerSecond)) true))

(fn ConstructionScript)