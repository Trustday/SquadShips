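; Flying tutorial enemy that patrols between four target points and attacks the player on sight.
; Tick forces a constant forward speed and steers by facing the current waypoint, switching to the next within a set distance.
; Pawn sensing triggers a timed chase state that faces BP_Main and fires projectiles with sound after a delay.
; On destruction it decrements the GameMode's tutorial enemy count and increments the GameInstance's kill tally.
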(event OnSeePawn(PawnSensing)
  (params (Pawn :type Pawn%20Object%20Reference))
  (Utilities|Casting|CastToBP_Main Pawn)
  (Utilities|FlowControl|Sequence
    (:then_0
      (Variables|Default|SetEstado 1))
    (:then_1
      (Utilities|FlowControl|Delay 3.0)
      (Variables|Default|SetEstado 0))))

(event Custom|RestarEnemigos
  ;[1 1 1] Restar Enemigos
  (bind _asbp_game_mode (Utilities|Casting|CastToBP_GameMode (Game|GetGameMode)))
  (Math|Integer|DecrementInt (Variables|/Game/Blueprint/GameMode/BP_GameMode.BP_GameMode_C|GetTuto1FlyingEnemies _asbp_game_mode)))

(event Custom|Siguiendo
  (bind _asbp_main (Utilities|Casting|CastToBP_Main (Game|GetPlayerCharacter 0)))
  (Transformation|SetActorRotation (Math|Rotator|FindLookatRotation (Transformation|GetWorldLocation (Variables|Default|GetSphere)) (Transformation|GetWorldLocation (Variables|/Game/Blueprint/BP_Main.BP_Main_C|GetMain_Target _asbp_main)))))

(event Custom|Disparar
  (Game|SpawnActorfromClass "/Game/Blueprint/BP_2_Primario.BP_2_Primario_C" (Transformation|GetWorldTransform (Variables|Default|GetSphere)) "Undefined" 0 0)
  (Audio|PlaySoundatLocation "/Game/Audio/Au_enemyShoot.Au_enemyShoot" (Transformation|GetActorLocation)) ; Play firing sound
)

(event Custom|Patrol
  (bind _target1 (Variables|Default|GetTarget1))
  (bind _target2 (Variables|Default|GetTarget2))
  (bind _spritecomponent (Variables|/Script/Engine.TargetPoint|GetSpriteComponent _target2))
  (bind _spritecomponent_2 (Variables|/Script/Engine.TargetPoint|GetSpriteComponent _target1))
  (bind _returnvalue (Transformation|GetWorldLocation _spritecomponent_2))
  (bind _returnvalue_2 (Transformation|GetWorldLocation _spritecomponent))
  (Variables|Default|SetPatrullando false)
  (Transformation|SetActorRotation (Math|Rotator|FindLookatRotation (Transformation|GetWorldLocation (Variables|Default|GetSphere)) _returnvalue))
  (AI|AIMoveTo self _returnvalue (Variables|Default|GetTarget1) 5.0 true
    (:OnSuccess
      (Transformation|SetActorRotation (Math|Rotator|FindLookatRotation (Transformation|GetWorldLocation (Variables|Default|GetSphere)) _returnvalue_2))
      (AI|AIMoveTo self _returnvalue_2 (Variables|Default|GetTarget2) 5.0 true
        (:OnSuccess
          (Variables|Default|SetPatrullando true)
          (CallFunction|Patrol))))))

(event EventDestroyed
  ;[1 1 1] Al destruir
  (CallFunction|RestarEnemigos)
  ;[1 1 1] Sumar uno a Enemies killed
  (bind _asglobal_game_instance (Utilities|Casting|CastToGlobalGameInstance (Game|GetGameInstance)))
  (Math|Integer|IncrementInt (Variables|/Game/Blueprint/GameMode/GlobalGameInstance.GlobalGameInstance_C|GetenemiesKilled _asglobal_game_instance)))

(event EventTick
  (params (DeltaSeconds :type Float%20%28single-precision%29))
  (Variables|Default|SetCurrent%20forward%20speed 2.5e+03)
  (|CallParentFunction DeltaSeconds)
  (switch int (Variables|Default|GetEstado)
    (:0
      (switch int (Variables|Default|GetTarget)
        (:0
          (Transformation|SetActorRotation (Math|Rotator|FindLookatRotation (Transformation|GetWorldLocation (Variables|Default|GetSphere)) (Transformation|GetWorldLocation (Variables|/Script/Engine.TargetPoint|GetSpriteComponent (Variables|Default|GetTarget1)))))
          (if (Math|Vector|Equal(Vector) (Transformation|GetWorldLocation (Variables|/Script/Engine.Actor|GetRootComponent (Variables|Default|GetTarget1))) (Transformation|GetWorldLocation (Variables|Default|GetDefaultSceneRoot)) 5e+02)
            (Variables|Default|SetTarget 1)))
        (:1
          (Transformation|SetActorRotation (Math|Rotator|FindLookatRotation (Transformation|GetWorldLocation (Variables|Default|GetSphere)) (Transformation|GetWorldLocation (Variables|/Script/Engine.Actor|GetRootComponent (Variables|Default|GetTarget2)))))
          (if (Math|Vector|Equal(Vector) (Transformation|GetWorldLocation (Variables|/Script/Engine.Actor|GetRootComponent (Variables|Default|GetTarget2))) (Transformation|GetWorldLocation (Variables|Default|GetDefaultSceneRoot)) 5e+02)
            (Variables|Default|SetTarget 2)))
        (:2
          (Transformation|SetActorRotation (Math|Rotator|FindLookatRotation (Transformation|GetWorldLocation (Variables|Default|GetSphere)) (Transformation|GetWorldLocation (Variables|/Script/Engine.Actor|GetRootComponent (Variables|Default|GetTarget3)))))
          (if (Math|Vector|Equal(Vector) (Transformation|GetWorldLocation (Variables|/Script/Engine.Actor|GetRootComponent (Variables|Default|GetTarget3))) (Transformation|GetWorldLocation (Variables|Default|GetDefaultSceneRoot)) 5e+02)
            (Variables|Default|SetTarget 3)))
        (:3
          (Transformation|SetActorRotation (Math|Rotator|FindLookatRotation (Transformation|GetWorldLocation (Variables|Default|GetSphere)) (Transformation|GetWorldLocation (Variables|/Script/Engine.Actor|GetRootComponent (Variables|Default|GetTarget4)))))
          (if (Math|Vector|Equal(Vector) (Transformation|GetWorldLocation (Variables|/Script/Engine.Actor|GetRootComponent (Variables|Default|GetTarget4))) (Transformation|GetWorldLocation (Variables|Default|GetDefaultSceneRoot)) 5e+02)
            (Variables|Default|SetTarget 0)))))
    (:1
      (CallFunction|Siguiendo)
      (Utilities|FlowControl|Delay 2.0)
      (CallFunction|Disparar))))

(fn ConstructionScript)