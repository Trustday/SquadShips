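; BP_ene_Mov is a moving enemy plane that flies forward, rams the player and can be destroyed by damage.
; Tick applies a swept forward offset and local roll, pitch and yaw rotation from speed variables that this graph never changes.
; Hitting BP_Main deals fixed damage and removes the enemy without explosion or kill credit.
; Lethal damage spawns an explosion with sound, increments EnemiesKilled in GlobalGameInstance and destroys it.
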(event EventTick
  (params (DeltaSeconds :type Float%20%28single-precision%29))
  (bind _returnvalue (Utilities|Time|GetWorldDeltaSeconds))
  ;[1 1 1] ON TICK: Apply forward speed and steering rotation
  (Transformation|AddActorLocalOffset (Math|Vector|MakeVector (* DeltaSeconds (Variables|Default|GetCurrent%20forward%20speed)) 0.0 0.0) true false) ; Sweep plane forwards
  (Transformation|AddActorLocalRotation (Math|Rotator|MakeRotator (* _returnvalue (Variables|Default|GetCurrent%20roll%20speed)) (* _returnvalue (Variables|Default|GetCurrent%20pitch%20speed)) (* _returnvalue (Variables|Default|GetCurrent%20yaw%20speed))) false false))

(event Game|Damage|EventAnyDamage
  (params (Damage :type Float%20%28single-precision%29) (DamageType :type Damage%20Type%20Object%20Reference) (InstigatedBy :type Controller%20Object%20Reference) (DamageCauser :type Actor%20Object%20Reference))
  (bind _returnvalue (Transformation|GetActorLocation))
  ;[1 1 1] Aplicar Daño
  (bind _output_get (Variables|Default|SetLife (- (Variables|Default|GetLife) Damage)))
  (if (<= _output_get 0.0)
    (Effects|SpawnEmitteratLocation "/Game/StarterContent/Particles/P_Explosion.P_Explosion" _returnvalue)
    (Audio|PlaySoundatLocation "/Game/StarterContent/Audio/Explosion01.Explosion01" _returnvalue)
    ;;[1 1 1] Sumar uno a Enemies killed
    (bind _asglobal_game_instance (Utilities|Casting|CastToGlobalGameInstance (Game|GetGameInstance)))
    (Math|Integer|IncrementInt (Variables|/Game/Blueprint/GameMode/GlobalGameInstance.GlobalGameInstance_C|GetenemiesKilled _asglobal_game_instance)
      (:%20%20
        (Actor|DestroyActor)))))

(event Collision|EventHit
  (params (MyComp :type Primitive%20Component%20Object%20Reference) (Other :type Actor%20Object%20Reference) (OtherComp :type Primitive%20Component%20Object%20Reference) (bSelfMoved :type Boolean) (HitLocation :type Vector :default "0, 0, 0") (HitNormal :type Vector :default "0, 0, 0") (NormalImpulse :type Vector :default "0, 0, 0") (Hit :type Hit%20Result%20Structure%20%28by%20ref%29))
  ;[1 1 1] Detectar Daño
  (bind _asbp_main (Utilities|Casting|CastToBP_Main (.HitActor (Collision|BreakHitResult Hit))))
  (Game|Damage|ApplyDamage _asbp_main 75.0 0 0)
  (Actor|DestroyActor))

(fn ConstructionScript)