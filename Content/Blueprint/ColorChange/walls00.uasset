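; Tutorial environment actor (walls00) that changes its Cube's appearance when the Room 1 missions are complete.
; Tick checks two BP_GameMode completion flags while the UnaVezCambio guard is true, then branches on actor tags.
; Room1 actors get a green grid material, while Door1 actors get strong green and lose collision.
; Only the door branch clears the guard, so Room1 actors reapply their material every frame.
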(event EventBeginPlay)

(event Collision|EventActorBeginOverlap
  (params (OtherActor :type Actor%20Object%20Reference)))

(event EventTick
  (params (DeltaSeconds :type Float%20%28single-precision%29))
  ;[1 1 1] Cambio material ROOM 1 al completar misión
  (if (Variables|Default|GetunaVezCambio)
    (bind _asbp_game_mode (Utilities|Casting|CastToBP_GameMode (Game|GetGameMode)))
    (if (and (Variables|/Game/Blueprint/GameMode/BP_GameMode.BP_GameMode_C|GetmissionCom_tuto1_room1_0 _asbp_game_mode) (Variables|/Game/Blueprint/GameMode/BP_GameMode.BP_GameMode_C|GetmissionCom_tuto1_room1_1 _asbp_game_mode))
      (if (Actor|ActorHasTag "Room1")
        (Rendering|Material|SetMaterial (Variables|Default|GetCube) 0 "/Game/Meshes/Materials/GridGreen.GridGreen")
        (else
          ;[1 1 1] Cambio material PUERTAS al completar misión
          (if (Actor|ActorHasTag "Door1")
            (Rendering|Material|SetMaterial (Variables|Default|GetCube) 0 "/Game/Meshes/Materials/MAT_Green_Strong.MAT_Green_Strong")
            (Collision|SetCollisionEnabled (Variables|Default|GetCube) "NoCollision")
            (Variables|Default|SetunaVezCambio false)))))))

(fn ConstructionScript)