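; BP_Objective_Sequence0 is a collectible objective, with star-pickup audio, that counts down the remaining Llaves (keys) in BP_GameMode.
; Any actor overlap plays the pickup sound at its location, decrements that counter and destroys the objective.
; On end overlap, a counter at zero or below triggers the mini-quest completion sound, gated by the UnaVezOverlap flag to play once per instance.
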(event EventBeginPlay)

(event Collision|EventActorBeginOverlap
  (params (OtherActor :type Actor%20Object%20Reference))
  ;[1 1 1] Disminuir variable al Overlap
  (bind _asbp_game_mode (Utilities|Casting|CastToBP_GameMode (Game|GetGameMode)))
  (Audio|PlaySoundatLocation "/Game/Audio/Au_starOverlap.Au_starOverlap" (Transformation|GetActorLocation))
  (Variables|/Game/Blueprint/BP_GameMode.BP_GameMode_C|SetLlaves _asbp_game_mode (- (Variables|/Game/Blueprint/BP_GameMode.BP_GameMode_C|GetLlaves _asbp_game_mode) 1))
  (Actor|DestroyActor))

(event EventTick
  (params (DeltaSeconds :type Float%20%28single-precision%29)))

(event Collision|EventActorEndOverlap
  (params (OtherActor :type Actor%20Object%20Reference))
  ;[1 1 1] Sonido al completar estrellas
  (if (<= (Variables|/Game/Blueprint/BP_GameMode.BP_GameMode_C|GetLlaves (stale Collision|EventActorBeginOverlap _asbp_game_mode)) 0)
    (if (Variables|Default|Getuna_vez_overlap)
      (Variables|Default|Setuna_vez_overlap false)
      (Audio|PlaySoundatLocation "/Game/Audio/Au_miniQuestComplete.Au_miniQuestComplete" (Transformation|GetActorLocation)))))

(fn ConstructionScript)