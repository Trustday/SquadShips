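; BP_SequenceObjectGoal is the goal actor that triggers victory and appears when the quest is complete.
; Each Tick it hides itself unless the game mode's Llaves and Objetivos counters are both zero.
; On overlap, if the player character is a FlyingPawn, it pauses the game and shows BP_Win with UI-only input and cursor.
; The overlap checks neither the overlapping actor nor the counters, and hiding leaves collision untouched.
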(event EventTick
  (params (DeltaSeconds :type Float%20%28single-precision%29))
  ;[1 1 1] Spam del Actor al completar la Quest
  (Rendering|SetActorHiddenInGame true)
  (bind _asbp_game_mode (Utilities|Casting|CastToBP_GameMode (Game|GetGameMode)))
  (Rendering|SetActorHiddenInGame (not (and (== (Variables|/Game/Blueprint/BP_GameMode.BP_GameMode_C|GetLlaves _asbp_game_mode) 0) (== (Variables|/Game/Blueprint/BP_GameMode.BP_GameMode_C|GetObjetivos _asbp_game_mode) 0)))))

(event Collision|EventActorBeginOverlap
  (params (OtherActor :type Actor%20Object%20Reference))
  (bind _returnvalue (Game|GetPlayerController 0))
  ;[1 1 1] Menu de Victoria
  (Utilities|Casting|CastToFlyingPawn (Game|GetPlayerCharacter 0))
  (Game|SetGamePaused true)
  (bind _returnvalue_2 (UserInterface|CreateWidget "/Game/UI/BP_Win.BP_Win_C"))
  (UserInterface|Viewport|AddtoViewport _returnvalue_2 0)
  (Input|SetInputModeUIOnly _returnvalue 0 "DoNotLock")
  (Variables|/Script/Engine.PlayerController|SetbShowMouseCursor _returnvalue true))

(fn ConstructionScript)