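; Enemy turret that spins in yaw until PawnSensing spots the player (BP_Main).
; On each sighting it aims at the player's MainTarget and fires BP_2_Primario, resuming rotation after a delay.
; Lethal damage decrements the game mode's Tuto1Turrets and explodes it.
; Colliding with the player deals damage, destroys the turret and increments EnemiesKilled, without updating Tuto1Turrets.
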(event OnSeePawn(PawnSensing)
  (params (Pawn :type Pawn%20Object%20Reference))
  ;[1 1 1] Disparo Torreta
  (Utilities|FlowControl|Sequence
    (:then_0
      (Variables|Default|SetNo_Viendo false)
      (bind _asbp_main (Utilities|Casting|CastToBP_Main Pawn))
      (Transformation|SetActorRotation (Math|Rotator|FindLookatRotation (Transformation|GetWorldLocation (Variables|Default|GetSphere1)) (Transformation|GetWorldLocation (Variables|/Game/Blueprint/BP_Main.BP_Main_C|GetMain_Target _asbp_main))))
      (Game|SpawnActorfromClass "/Game/Blueprint/BP_2_Primario.BP_2_Primario_C" (Transformation|GetWorldTransform (Variables|Default|GetSphere1)) "Undefined" 0 0)
      (Audio|PlaySoundatLocation "/Game/Audio/Au_enemyShoot.Au_enemyShoot" (Transformation|GetActorLocation)) ; Play firing sound
    )
    (:then_1
      (Utilities|FlowControl|Delay 0.5)
      (Variables|Default|SetNo_Viendo true))))

(event OnComponentBeginOverlap(Vision)
  (params (OverlappedComponent :type Primitive%20Component%20Object%20Reference) (OtherActor :type Actor%20Object%20Reference) (OtherComp :type Primitive%20Component%20Object%20Reference) (OtherBodyIndex :type Integer) (bFromSweep :type Boolean) (SweepResult :type Hit%20Result%20Structure%20%28by%20ref%29))
  ;[1 1 1] Detectar Vision
)

(event OnComponentEndOverlap(Vision)
  (params (OverlappedComponent :type Primitive%20Component%20Object%20Reference) (OtherActor :type Actor%20Object%20Reference) (OtherComp :type Primitive%20Component%20Object%20Reference) (OtherBodyIndex :type Integer))
  ;[1 1 1] Detectar Vision
)

(event Custom|RestarEnemigos
  ;[1 1 1] Restar Enemigos
  (bind _asbp_game_mode (Utilities|Casting|CastToBP_GameMode (Game|GetGameMode)))
  (Variables|/Game/Blueprint/GameMode/BP_GameMode.BP_GameMode_C|SetTuto1Turrets _asbp_game_mode (- (Variables|/Game/Blueprint/GameMode/BP_GameMode.BP_GameMode_C|GetTuto1Turrets _asbp_game_mode) 1)))

(event EventTick
  (params (DeltaSeconds :type Float%20%28single-precision%29))
  ;[1 1 1] Comportamiento de rotacion
  (if (Variables|Default|GetNo_Viendo)
    (Transformation|SetActorRotation (Math|Rotator|MakeRotator 0.0 0.0 (+ (.yaw (Transformation|GetActorRotation)) 5.0)))))

(event Game|Damage|EventAnyDamage
  (params (Damage :type Float%20%28single-precision%29) (DamageType :type Damage%20Type%20Object%20Reference) (InstigatedBy :type Controller%20Object%20Reference) (DamageCauser :type Actor%20Object%20Reference))
  (bind _returnvalue (Transformation|GetActorLocation))
  ;[1 1 1] Aplicar Daño
  (bind _output_get (Variables|Default|SetLife (- (Variables|Default|GetLife) Damage)))
  (if (<= _output_get 0.0)
    (CallFunction|RestarEnemigos)
    (Effects|SpawnEmitteratLocation "/Game/StarterContent/Particles/P_Explosion.P_Explosion" _returnvalue)
    (Audio|PlaySoundatLocation "/Game/StarterContent/Audio/Explosion01.Explosion01" _returnvalue)
    (Actor|DestroyActor)))

(event Collision|EventHit
  (params (MyComp :type Primitive%20Component%20Object%20Reference) (Other :type Actor%20Object%20Reference) (OtherComp :type Primitive%20Component%20Object%20Reference) (bSelfMoved :type Boolean) (HitLocation :type Vector :default "0, 0, 0") (HitNormal :type Vector :default "0, 0, 0") (NormalImpulse :type Vector :default "0, 0, 0") (Hit :type Hit%20Result%20Structure%20%28by%20ref%29))
  ;[1 1 1] Detectar Daño
  (bind _asbp_main (Utilities|Casting|CastToBP_Main (.HitActor (Collision|BreakHitResult Hit))))
  (Game|Damage|ApplyDamage _asbp_main 75.0 0 0)
  (Actor|DestroyActor)
  ;[1 1 1] Sumar uno a Enemies killed
  (bind _asglobal_game_instance (Utilities|Casting|CastToGlobalGameInstance (Game|GetGameInstance)))
  (Math|Integer|IncrementInt (Variables|/Game/Blueprint/GameMode/GlobalGameInstance.GlobalGameInstance_C|GetenemiesKilled _asglobal_game_instance)))

(fn ConstructionScript)