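; BP_PortalOrange is a portal actor that switches the BP_Main ship to its orange state, Estado2, when the ship overlaps it.
; On overlap, it swaps the ship's mesh material to StrongOrange, plays a mode-change sound at the ship and sets ShipState, skipping ships already in that state.
; Tick spins the portal by a fixed local rotation each frame, so the spin speed depends on frame rate.
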(event EventBeginPlay)

(event Collision|EventActorBeginOverlap
  (params (OtherActor :type Actor%20Object%20Reference))
  (bind _asbp_main (Utilities|Casting|CastToBP_Main OtherActor))
  (if (!= (Variables|/Game/Blueprint/BP_Main.BP_Main_C|GetShipState _asbp_main) (Variables|Default|GetEstado2))
    (Rendering|Material|SetMaterial (Variables|/Script/Engine.Character|GetMesh _asbp_main) 0 "/Game/Meshes/Materials/strongOrange.strongOrange")
    (Audio|PlaySoundatLocation "/Game/Audio/Au_changeMode.Au_changeMode" (Transformation|GetActorLocation _asbp_main))
    (Variables|/Game/Blueprint/BP_Main.BP_Main_C|SetShipState _asbp_main (Variables|Default|GetEstado2))))

(event EventTick
  (params (DeltaSeconds :type Float%20%28single-precision%29))
  (Transformation|AddActorLocalRotation "0, 0,2.000000" false false))

(fn ConstructionScript)