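; BP_PortalStandard is a spinning portal that switches a FlyingPawn passing through it to ship state Estado1.
; On actor overlap, a pawn not already in that state gets the Pod_blinn material on its mesh, a mode-change sound at its location and the new state.
; Tick applies a fixed local rotation each frame without delta-time scaling, so spin speed depends on frame rate.
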(event EventBeginPlay)

(event Collision|EventActorBeginOverlap
  (params (OtherActor :type Actor%20Object%20Reference))
  (bind _asflying_pawn (Utilities|Casting|CastToFlyingPawn OtherActor))
  (if (!= (Variables|/Game/Blueprint/FlyingPawn.FlyingPawn_C|GetShipState _asflying_pawn) (Variables|Default|GetEstado1))
    (Rendering|Material|SetMaterial (Variables|/Script/Engine.Character|GetMesh _asflying_pawn) 0 "/Game/Flying/Meshes/pod_blinn.pod_blinn")
    (Audio|PlaySoundatLocation "/Game/Audio/Au_changeMode.Au_changeMode" (Transformation|GetActorLocation _asflying_pawn))
    (Variables|/Game/Blueprint/FlyingPawn.FlyingPawn_C|SetShipState _asflying_pawn (Variables|Default|GetEstado1))))

(event EventTick
  (params (DeltaSeconds :type Float%20%28single-precision%29))
  (Transformation|AddActorLocalRotation "0, 0,2.000000" false false))

(fn ConstructionScript)