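; BP_PowerUp_Speed is a speed power-up that changes the forward speed of the BP_Main ship on overlap.
; When NewSpeed differs from the ship's DefaultSpeed, it writes NewSpeed to both CurrentForwardSpeed and DefaultSpeed, so it sets no timer and stays in place.
; An unconnected branch that would switch ship state, material and play a mode-change sound never runs.
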(event EventBeginPlay)

(event Collision|EventActorBeginOverlap
  (params (OtherActor :type Actor%20Object%20Reference))
  (bind _asbp_main (Utilities|Casting|CastToBP_Main OtherActor))
  (if (!= (Variables|Default|GetnewSpeed) (Variables|/Game/Blueprint/BP_Main.BP_Main_C|GetDefaultSpeed _asbp_main))
    (bind _output_get (Variables|/Game/Blueprint/BP_Main.BP_Main_C|SetCurrent%20forward%20speed _asbp_main (Variables|Default|GetnewSpeed)))
    (Variables|/Game/Blueprint/BP_Main.BP_Main_C|SetDefaultSpeed _asbp_main _output_get)))

(event EventTick
  (params (DeltaSeconds :type Float%20%28single-precision%29)))

(fn ConstructionScript)