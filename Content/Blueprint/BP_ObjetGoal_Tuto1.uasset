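; Tutorial 1 goal object that appears once the quest is complete and triggers victory when the player reaches it.
; It starts hidden without collision, then polls BP_GameMode on Tick, enabling itself when both turret and flying-enemy counters reach zero or below.
; A one-shot flag gates the quest-complete sound.
; Overlap pauses the game, shows the W_Victory widget and switches to UI-only input with a cursor.
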(event EventTick
  (params (DeltaSeconds :type Float%20%28single-precision%29))
  ;[1 1 1] Spawn del Actor al completar la Quest
  (bind _asbp_game_mode (Utilities|Casting|CastToBP_GameMode (Game|GetGameMode)))
  (Rendering|SetActorHiddenInGame (Math|Boolean|NANDBoolean (<= (Variables|/Game/Blueprint/GameMode/BP_GameMode.BP_GameMode_C|GetTuto1Turrets _asbp_game_mode) 0) (<= (Variables|/Game/Blueprint/GameMode/BP_GameMode.BP_GameMode_C|GetTuto1FlyingEnemies _asbp_game_mode) 0)))
  (Collision|SetActorEnableCollision (not (Math|Boolean|NANDBoolean (<= (Variables|/Game/Blueprint/GameMode/BP_GameMode.BP_GameMode_C|GetTuto1Turrets _asbp_game_mode) 0) (<= (Variables|/Game/Blueprint/GameMode/BP_GameMode.BP_GameMode_C|GetTuto1FlyingEnemies _asbp_game_mode) 0))))
  ;[1 1 1] Sonido Quest complete
  (if (not (Math|Boolean|NANDBoolean (<= (Variables|/Game/Blueprint/GameMode/BP_GameMode.BP_GameMode_C|GetTuto1Turrets _asbp_game_mode) 0) (<= (Variables|/Game/Blueprint/GameMode/BP_GameMode.BP_GameMode_C|GetTuto1FlyingEnemies _asbp_game_mode) 0)))
    (if (Variables|Default|Getuna_vez)
      (Variables|Default|Setuna_vez false)
      (Audio|PlaySoundatLocation "/Game/Audio/Au_QuestComplete.Au_QuestComplete" (Transformation|GetActorLocation)))))

(event Collision|EventActorBeginOverlap
  (params (OtherActor :type Actor%20Object%20Reference))
  (bind _returnvalue (Game|GetPlayerController 0))
  ;[1 1 1] Menu de Victoria
  (Utilities|Casting|CastToBP_Main (Game|GetPlayerCharacter 0))
  (Game|SetGamePaused true)
  (bind _returnvalue_2 (UserInterface|CreateWidget "/Game/UI/W_Victory.W_Victory_C"))
  (UserInterface|Viewport|AddtoViewport _returnvalue_2 0)
  (Input|SetInputModeUIOnly _returnvalue 0 "DoNotLock")
  (Variables|/Script/Engine.PlayerController|SetbShowMouseCursor _returnvalue true))

(event EventBeginPlay
  ;[1 1 1] Desactiva colisión con objetivo final
  (Rendering|SetActorHiddenInGame true)
  (Collision|SetActorEnableCollision false))

(fn ConstructionScript)