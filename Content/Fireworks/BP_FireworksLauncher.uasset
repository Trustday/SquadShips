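; Fireworks launcher actor that spawns BP_Fireworks_Shell actors to produce a fireworks display.
; Both Tick and the LaunchShell event feed the same spawn, so a shell launches every frame as well as on each call.
; Shells start at Arrow1 with its rotation randomly offset within RandomAngle.
; The launcher passes its motion, lifetime and burst settings to each shell, with a randomly picked burst particle system.
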(event Custom|LaunchShell
  (bind _arrow1 (Variables|Default|GetArrow1))
  (bind _burstparticlesystems (Variables|BurstProperties|GetBurstParticleSystems))
  (bind _returnvalue (Transformation|GetWorldTransform _arrow1))
  (bind (_location _rotation) (Math|Transform|BreakTransform _returnvalue))
  (Game|SpawnActorfromClass "/Game/Fireworks/BP_Fireworks_Shell.BP_Fireworks_Shell_C" (Math|Transform|MakeTransform _location (Math|Rotator|CombineRotators _rotation (Math|Rotator|MakeRotator (Math|Random|RandomFloatinRange (* (Variables|Default|GetRandomAngle) -1.0) (Variables|Default|GetRandomAngle)) (Math|Random|RandomFloatinRange (* (Variables|Default|GetRandomAngle) -1.0) (Variables|Default|GetRandomAngle)) (Math|Random|RandomFloatinRange (* (Variables|Default|GetRandomAngle) -1.0) (Variables|Default|GetRandomAngle))))) "AlwaysSpawn" 0 (Variables|ShellProperties|GetMaxRotationSpeed) (Variables|ShellProperties|GetMinRotationSpeed) (Variables|ShellProperties|GetMaxLaunchVelocity) (Variables|ShellProperties|GetMinLaunchVelocity) (Variables|ShellProperties|GetShellMaxLife) (Variables|ShellProperties|GetShellminLife) (Variables|BurstProperties|GetMaxBurstTime) (Variables|BurstProperties|GetMinBurstTime) (Utilities|Array|Get(acopy) _burstparticlesystems (Math|Random|RandomInteger (Utilities|Array|Length _burstparticlesystems))) (Variables|ShellProperties|GetShellParticleSystem) false (Variables|BurstProperties|GetNumberOfBursts) (Variables|BurstProperties|GetSecondaryBurstDelay) 0))

(event EventTick
  (params (DeltaSeconds :type Float%20%28single-precision%29))
  (bind _arrow1 (Variables|Default|GetArrow1))
  (bind _burstparticlesystems (Variables|BurstProperties|GetBurstParticleSystems))
  (bind _returnvalue (Transformation|GetWorldTransform _arrow1))
  (bind (_location _rotation) (Math|Transform|BreakTransform _returnvalue))
  (Game|SpawnActorfromClass "/Game/Fireworks/BP_Fireworks_Shell.BP_Fireworks_Shell_C" (Math|Transform|MakeTransform _location (Math|Rotator|CombineRotators _rotation (Math|Rotator|MakeRotator (Math|Random|RandomFloatinRange (* (Variables|Default|GetRandomAngle) -1.0) (Variables|Default|GetRandomAngle)) (Math|Random|RandomFloatinRange (* (Variables|Default|GetRandomAngle) -1.0) (Variables|Default|GetRandomAngle)) (Math|Random|RandomFloatinRange (* (Variables|Default|GetRandomAngle) -1.0) (Variables|Default|GetRandomAngle))))) "AlwaysSpawn" 0 (Variables|ShellProperties|GetMaxRotationSpeed) (Variables|ShellProperties|GetMinRotationSpeed) (Variables|ShellProperties|GetMaxLaunchVelocity) (Variables|ShellProperties|GetMinLaunchVelocity) (Variables|ShellProperties|GetShellMaxLife) (Variables|ShellProperties|GetShellminLife) (Variables|BurstProperties|GetMaxBurstTime) (Variables|BurstProperties|GetMinBurstTime) (Utilities|Array|Get(acopy) _burstparticlesystems (Math|Random|RandomInteger (Utilities|Array|Length _burstparticlesystems))) (Variables|ShellProperties|GetShellParticleSystem) false (Variables|BurstProperties|GetNumberOfBursts) (Variables|BurstProperties|GetSecondaryBurstDelay) 0))

(fn ConstructionScript)