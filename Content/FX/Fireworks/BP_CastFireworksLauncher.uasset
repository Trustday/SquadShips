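; Fireworks launcher actor that celebrates completion of two tutorial room missions tracked in BP_GameMode.
; Tick moves it to the game mode's fireworks position when flagged, otherwise waits for both missions.
; It then spawns one BP_Fireworks_Shell from Arrow1 with randomized rotation and configured launch, life and burst settings, destroying itself ten seconds later.
; LaunchShell triggers the same sequence directly, bypassing the mission and one-shot checks.
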(event Custom|LaunchShell
  (bind _arrow1 (Variables|Default|GetArrow1))
  (bind _returnvalue (Transformation|GetWorldTransform _arrow1))
  (bind (_location _rotation) (Math|Transform|BreakTransform _returnvalue))
  (Game|SpawnActorfromClass "/Game/FX/Fireworks/BP_Fireworks_Shell.BP_Fireworks_Shell_C" (Math|Transform|MakeTransform _location (Math|Rotator|CombineRotators _rotation (Math|Rotator|MakeRotator (Math|Random|RandomFloatinRange (* (Variables|Default|GetRandomAngle) -1.0) (Variables|Default|GetRandomAngle)) (Math|Random|RandomFloatinRange (* (Variables|Default|GetRandomAngle) -1.0) (Variables|Default|GetRandomAngle)) (Math|Random|RandomFloatinRange (* (Variables|Default|GetRandomAngle) -1.0) (Variables|Default|GetRandomAngle))))) "AlwaysSpawn" 0 (Variables|ShellProperties|GetMaxRotationSpeed) (Variables|ShellProperties|GetMinRotationSpeed) (Variables|ShellProperties|GetMaxLaunchVelocity) (Variables|ShellProperties|GetMinLaunchVelocity) (Variables|ShellProperties|GetShellMaxLife) (Variables|ShellProperties|GetShellminLife) (Variables|BurstProperties|GetMaxBurstTime) (Variables|BurstProperties|GetMinBurstTime) 0 (Variables|ShellProperties|GetShellParticleSystem) false (Variables|BurstProperties|GetNumberOfBursts) (Variables|BurstProperties|GetSecondaryBurstDelay) 0)
  (Variables|Default|SetunaVez false)
  (Utilities|FlowControl|Delay 1e+01)
  (Actor|DestroyActor))

(event EventTick
  (params (DeltaSeconds :type Float%20%28single-precision%29))
  (bind _arrow1 (Variables|Default|GetArrow1))
  (bind _returnvalue (Transformation|GetWorldTransform _arrow1))
  (bind (_location _rotation) (Math|Transform|BreakTransform _returnvalue))
  ;[1 1 1] Si se completan las dos quests
  (bind _asbp_game_mode (Utilities|Casting|CastToBP_GameMode (Game|GetGameMode)))
  (if (Variables|/Game/Blueprint/GameMode/BP_GameMode.BP_GameMode_C|GetsetFireworksPosition _asbp_game_mode)
    (Transformation|SetActorLocation (Variables|/Game/Blueprint/GameMode/BP_GameMode.BP_GameMode_C|GetfireworksPosition _asbp_game_mode) false false)
    (Variables|/Game/Blueprint/GameMode/BP_GameMode.BP_GameMode_C|SetsetFireworksPosition _asbp_game_mode false) ; Vaiable para posicionar los fuegos artificiales
    (elif (and (Variables|/Game/Blueprint/GameMode/BP_GameMode.BP_GameMode_C|GetmissionCom_tuto1_room2_0 _asbp_game_mode) (Variables|/Game/Blueprint/GameMode/BP_GameMode.BP_GameMode_C|GetmissionCom_tuto1_room2_1 _asbp_game_mode))
      (if (Variables|Default|GetunaVez)
        (Game|SpawnActorfromClass "/Game/FX/Fireworks/BP_Fireworks_Shell.BP_Fireworks_Shell_C" (Math|Transform|MakeTransform _location (Math|Rotator|CombineRotators _rotation (Math|Rotator|MakeRotator (Math|Random|RandomFloatinRange (* (Variables|Default|GetRandomAngle) -1.0) (Variables|Default|GetRandomAngle)) (Math|Random|RandomFloatinRange (* (Variables|Default|GetRandomAngle) -1.0) (Variables|Default|GetRandomAngle)) (Math|Random|RandomFloatinRange (* (Variables|Default|GetRandomAngle) -1.0) (Variables|Default|GetRandomAngle))))) "AlwaysSpawn" 0 (Variables|ShellProperties|GetMaxRotationSpeed) (Variables|ShellProperties|GetMinRotationSpeed) (Variables|ShellProperties|GetMaxLaunchVelocity) (Variables|ShellProperties|GetMinLaunchVelocity) (Variables|ShellProperties|GetShellMaxLife) (Variables|ShellProperties|GetShellminLife) (Variables|BurstProperties|GetMaxBurstTime) (Variables|BurstProperties|GetMinBurstTime) 0 (Variables|ShellProperties|GetShellParticleSystem) false (Variables|BurstProperties|GetNumberOfBursts) (Variables|BurstProperties|GetSecondaryBurstDelay) 0)
        (Variables|Default|SetunaVez false)
        (Utilities|FlowControl|Delay 1e+01)
        (Actor|DestroyActor)))))

(fn ConstructionScript)